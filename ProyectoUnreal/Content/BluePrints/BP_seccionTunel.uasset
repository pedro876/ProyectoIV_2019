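; Recyclable tunnel section holding a ring, a bomb and an obstacle as child actors, randomised at BeginPlay.
; When BP_nave overlaps DetectorRecolocar, the section jumps along negative Y by a distance scaled by the game mode's MaxModulos.
; Any overlap re-randomises the contents, with a flag telling the obstacle whether the game is starting.
; Ring and bomb independently pick one of nine target points, and each child runs its own randomiser.
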(event OnComponentBeginOverlap(detectorRecolocar)
  (params (OverlappedComponent :type Primitive%20Component%20Object%20Reference) (OtherActor :type Actor%20Object%20Reference) (OtherComp :type Primitive%20Component%20Object%20Reference) (OtherBodyIndex :type Integer) (bFromSweep :type Boolean) (SweepResult :type Hit%20Result%20Structure%20%28by%20ref%29))
  (CallFunction|FuncRecolocarModulo OtherActor)
  (CallFunction|FuncAleatorizarTodo false))

(event EventBeginPlay
  (CallFunction|FuncAleatorizarTodo true))

(event Collision|EventActorBeginOverlap
  (params (OtherActor :type Actor%20Object%20Reference)))

(event EventTick
  (params (DeltaSeconds :type Float%20%28single-precision%29)))

(fn ConstructionScript)

(fn FuncAleatorizarAroBomba
  (bind _targetpoint5 (Variables|Default|GettargetPoint5))
  (bind _targetpoint2 (Variables|Default|GettargetPoint2))
  (bind _bp_bomba (Variables|Default|Getbp_bomba))
  (bind _targetpoint3 (Variables|Default|GettargetPoint3))
  (bind _targetpoint4 (Variables|Default|GettargetPoint4))
  (bind _targetpoint1 (Variables|Default|GettargetPoint1))
  (bind _targetpoint6 (Variables|Default|GettargetPoint6))
  (bind _targetpoint7 (Variables|Default|GettargetPoint7))
  (bind _targetpoint8 (Variables|Default|GettargetPoint8))
  (bind _targetpoint9 (Variables|Default|GettargetPoint9))
  (bind _array (Utilities|Array|MakeArray _targetpoint5 _targetpoint2 _targetpoint3 _targetpoint4 _targetpoint1 _targetpoint6 _targetpoint7 _targetpoint8 _targetpoint9))
  (bind _returnvalue (Utilities|Array|Length _array))
  (Transformation|SetRelativeLocation (Variables|Default|Getbp_aro) (.Location (Math|Transform|BreakTransform (Transformation|GetRelativeTransform (Utilities|Array|Get(acopy) _array (Math|Random|RandomInteger _returnvalue))))) false false)
  (Transformation|SetRelativeLocation _bp_bomba (.Location (Math|Transform|BreakTransform (Transformation|GetRelativeTransform (Utilities|Array|Get(acopy) _array (Math|Random|RandomInteger _returnvalue))))) false false)
  (bind _asbp_bomba (Utilities|Casting|CastToBP_bomba (Variables|/Script/Engine.ChildActorComponent|GetChildActor _bp_bomba)))
  (Default|FuncAleatorizar _asbp_bomba))

(fn FuncAleatorizarTodo
  (params (inicioPartida :type Boolean))
  ;[1 1 1] Aleatorizar todo
  (CallFunction|FuncAleatorizarAroBomba)
  (bind _asbp_obstaculo (Utilities|Casting|CastToBP_Obstaculo (Variables|/Script/Engine.ChildActorComponent|GetChildActor (Variables|Default|Getbp_obstaculo))))
  (Default|FuncAleatorizar _asbp_obstaculo inicioPartida)
  (bind _asbp_aro (Utilities|Casting|CastToBP_aro (Variables|/Script/Engine.ChildActorComponent|GetChildActor (Variables|Default|Getbp_aro))))
  (Default|FuncAleatorizar _asbp_aro))

(fn FuncRecolocarModulo
  (params (actor :type Actor%20Object%20Reference))
  (bind _asbp_modo_juego (Utilities|Casting|CastToBP_modoJuego (Game|GetGameMode)))
  (Utilities|Casting|CastToBP_nave actor)
  (Transformation|SetActorLocation (Math|Vector|MakeVector 0.0 (+ (.y (Transformation|GetWorldLocation (Variables|Default|GetdetectorRecolocar))) (* -2e+03 (Math|Conversions|ToFloat(Integer) (Variables|/Game/BluePrints/BP_modoJuego.BP_modoJuego_C|GetmaxModulos _asbp_modo_juego)))) 0.0) false false))