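; BP_modoJuego, apparently the game mode, tracks the minimum spacing in modules between obstacles.
; FuncEmpezarContador starts counting, and each FuncAumentarContador call increments the counter until it reaches the minimum, then resets it and stops.
; Before each comparison, the minimum is recomputed from the player BP_nave's absolute MaxVelocidadY, scaled down and truncated, so gaps widen with that speed.
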(fn ConstructionScript)

(fn FuncAumentarContador
  ;[1 1 1] Si estoy contando modulos
  (if (Variables|Default|GetcontandoModulos)
    ;[1 1 1] Actualizamos el espacio mínimo entre obstáculos
    (CallFunction|FuncAumentarEspacioMin)
    (if (>= (Variables|Default|GetcontadorModulos) (Variables|Default|GetespacioMinModulos))
      ;[1 1 1] Si lo ha alcanzado, resetear el contador y dejar de contar módulos
      (Variables|Default|SetcontadorModulos 0)
      (Variables|Default|SetcontandoModulos false)
      (else
        ;[1 1 1] Si no lo ha alcanzado, aumentamos el contador
        (Math|Integer|IncrementInt (Variables|Default|GetcontadorModulos))))))

(fn FuncEmpezarContador
  ;[1 1 1] Empieza a contar módulos
  (Variables|Default|SetcontandoModulos true))

(fn FuncAumentarEspacioMin
  ;[1 1 1] Cada 10 unidades de velocidad, aumenta una unidad el espacio mínimo entre obstáculos
  (bind _asbp_nave (Utilities|Casting|CastToBP_nave (Game|Player|GetPlayerPawn 0)))
  (Variables|Default|SetespacioMinModulos (Math|Float|Truncate (/ (Math|Float|Absolute(Float) (Variables|/Game/BluePrints/BP_nave.BP_nave_C|GetmaxVelocidadY _asbp_nave)) 1e+03))))