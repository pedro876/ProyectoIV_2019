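; BP_camara is the game camera that follows the player's ship, BP_nave, at a fixed offset.
; On BeginPlay it caches the player pawn, stores the camera's initial offset from the ship's ColisionNave component and becomes the player's view target.
; Each tick it moves the camera component to the ship position plus that offset, clamping height between AlturaMinima and AlturaMaxima.
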(event EventTick
  (params (DeltaSeconds :type Float%20%28single-precision%29))
  (bind _jugador (Variables|Default|Getjugador))
  (bind _posicion (Variables|Default|Getposicion))
  (bind _colisionnave (Variables|/Game/BluePrints/BP_nave.BP_nave_C|GetcolisionNave _jugador))
  (bind _returnvalue (Transformation|GetWorldLocation _colisionnave))
  (bind _returnvalue_2 (+ _returnvalue _posicion))
  ;[1 1 1] Se asigna la posición de la cámara para que mantenga la distancia original
  (Transformation|SetWorldLocation (Variables|CameraActor|GetCameraComponent) (Math|Vector|MakeVector (.x _returnvalue_2) (.y _returnvalue_2) (Math|Float|Clamp(Float) (.z _returnvalue_2) (Variables|Default|GetalturaMinima) (Variables|Default|GetalturaMaxima))) false false))

(event EventBeginPlay
  ;[1 1 1] Se guarda una referencia al jugador
  (bind _asbp_nave (Utilities|Casting|CastToBP_nave (Game|Player|GetPlayerPawn 0)))
  (Variables|Default|Setjugador _asbp_nave)
  ;[1 1 1] Se guarda la posición relativa al jugador original de la nave
  (Variables|Default|Setposicion (- (Transformation|GetWorldLocation (Variables|CameraActor|GetCameraComponent)) (Transformation|GetWorldLocation (Variables|/Game/BluePrints/BP_nave.BP_nave_C|GetcolisionNave (Variables|Default|Getjugador)))))
  ;[1 1 1] Se asigna esta cámara por defecto para el juego
  (Game|Player|SetViewTargetwithBlend (Game|GetPlayerController 0) (Components|GetOwner (Variables|CameraActor|GetCameraComponent)) 0.0 "VTBlend_Linear" 0.0 false))

(fn ConstructionScript)