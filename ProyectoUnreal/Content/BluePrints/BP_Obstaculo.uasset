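; BP_Obstaculo is an obstacle actor that randomizes itself on BeginPlay and whenever its root component activates.
; FuncAleatorizar uses ProbabilidadDestruir to either deactivate the root component or call FuncAleatorizarMallaRot.
; That function gives the mesh a random quarter-turn pitch and one of three static meshes.
; Deactivation does not destroy or hide the actor, as the visibility and collision toggles are unconnected.
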(event OnComponentActivated(DefaultSceneRoot)
  (params (Component :type Actor%20Component%20Object%20Reference) (bReset :type Boolean))
  (CallFunction|FuncAleatorizar)
  (Development|PrintString "Aleatorizando"))

(event EventBeginPlay
  (CallFunction|FuncAleatorizar))

(fn ConstructionScript)

(fn FuncAleatorizarMallaRot
  (bind _malla_obstaculo (Variables|Default|Getmalla_obstaculo))
  (bind _malla_obstaculo_2 (Variables|Default|Getmalla_obstaculo))
  (bind _returnvalue (Transformation|GetRelativeTransform _malla_obstaculo_2))
  (bind (_location _rotation _scale) (Math|Transform|BreakTransform _returnvalue))
  (bind (_roll _pitch _yaw) (Math|Rotator|BreakRotator _rotation))
  ;[1 1 1] Rotación al azar
  (Transformation|SetRelativeTransform _malla_obstaculo (Math|Transform|MakeTransform _location (Math|Rotator|MakeRotator _roll (* (Math|Conversions|ToFloat(Integer) (Math|Random|RandomInteger 4)) 9e+01) _yaw) _scale) false false)
  ;[1 1 1] Obstáculo al azar
  (switch int (Math|Random|RandomInteger 3)
    (:Default
      (Components|StaticMesh|SetStaticMesh _malla_obstaculo "/Game/Geometria/obstaculos/obstaculo1.obstaculo1" :!label _label))
    (:0
      (goto _label))
    (:1
      (Components|StaticMesh|SetStaticMesh _malla_obstaculo "/Game/Geometria/obstaculos/obstaculo2.obstaculo2"))
    (:2
      (Components|StaticMesh|SetStaticMesh _malla_obstaculo "/Game/Geometria/obstaculos/obstaculo3.obstaculo3"))))

(fn FuncAleatorizar
  (if (< (Math|Random|RandomFloat) (Variables|Default|Getprobabilidad_destruir))
    (Components|Activation|SetActive (Variables|/Script/Engine.Actor|GetRootComponent (Components|GetOwner (Variables|Default|GetDefaultSceneRoot))) false false)
    (Development|PrintString "Desactivando")
    (else
      (CallFunction|FuncAleatorizarMallaRot))))