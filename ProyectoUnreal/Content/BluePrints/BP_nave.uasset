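; BP_nave is a physics-driven ship that constantly accelerates along negative Y while movement values steer it on the X and Z axes.
; Each Tick applies a mass-independent force to ColisionNave, subtracting current X and Z velocity so lateral motion is damped and settles toward input times VelocidadXz.
; FuncLimitarVelocidad then clamps Y velocity at MaxVelocidad.Y, leaving X and Z untouched.
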(event EventTick
  (params (DeltaSeconds :type Float%20%28single-precision%29))
  (bind _velocidad_xz (Variables|Default|Getvelocidad_xz))
  (bind _colisionnave (Variables|Default|GetcolisionNave))
  (bind _returnvalue (Transformation|GetComponentVelocity _colisionnave))
  (bind (_x _y _z) (Math|Vector|BreakVector _returnvalue))
  (Physics|AddForce (Variables|Default|GetcolisionNave) (- (Math|Vector|MakeVector (* (Input|AxisValues|Getmovimiento_horizontal) _velocidad_xz) -5e+02 (* _velocidad_xz (Input|AxisValues|Getmovimiento_vertical))) (Math|Vector|MakeVector _x 0.0 _z)) "None" true)
  (CallFunction|FuncLimitarVelocidad))

(fn ConstructionScript)

(fn FuncLimitarVelocidad
  (bind _maxvelocidad (Variables|Default|GetmaxVelocidad))
  (bind _colisionnave (Variables|Default|GetcolisionNave))
  (bind _returnvalue (Transformation|GetComponentVelocity _colisionnave))
  (bind _y (Math|Vector|BreakVector _maxvelocidad))
  (bind (_x _y_2 _z) (Math|Vector|BreakVector _returnvalue))
  (if (< _y_2 _y)
    (Physics|SetPhysicsLinearVelocity (Variables|Default|GetcolisionNave) (Math|Vector|MakeVector _x _y _z) false "None")))