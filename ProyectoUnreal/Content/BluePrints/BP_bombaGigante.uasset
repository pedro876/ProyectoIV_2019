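; BP_bombaGigante is a giant bomb that travels down the tunnel, clearing whatever it overlaps, until a lifetime timer destroys it.
; Each Tick grows the mesh uniformly up to a maximum, pulls it toward the tunnel's center and spins it.
; Forward movement adds the player ship's maximum speed, scaled by delta time, plus a fixed per-frame step.
; Overlaps kill enemies through a state change, destroy bullets, and hide obstacles with collision disabled.
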(event OnComponentBeginOverlap(colision)
  (params (OverlappedComponent :type Primitive%20Component%20Object%20Reference) (OtherActor :type Actor%20Object%20Reference) (OtherComp :type Primitive%20Component%20Object%20Reference) (OtherBodyIndex :type Integer) (bFromSweep :type Boolean) (SweepResult :type Hit%20Result%20Structure%20%28by%20ref%29))
  ;[1 1 1] Si colisiona con un enemigo, lo mata
  (bind _asbp_enemigo (Utilities|Casting|CastToBP_enemigo OtherActor)
    (:then
      (Default|FuncCambiarEstado _asbp_enemigo "NewEnumerator3"))
    (:CastFailed
      ;[1 1 1] Si colisiona con una bala la elimina
      (bind _asbp_bala (Utilities|Casting|CastToBP_bala OtherActor)
        (:then
          (Default|FuncMorir _asbp_bala))
        (:CastFailed
          ;[1 1 1] Si choca con un obstáculo lo quita del camino ocultándolo
          (bind _asbp_obstaculo (Utilities|Casting|CastToBP_Obstaculo OtherActor))
          (Rendering|SetActorHiddenInGame _asbp_obstaculo true)
          (Collision|SetActorEnableCollision _asbp_obstaculo false))))))

(event Custom|morir
  ;[1 1 1] Pasado cierto tiempo, la bomba gigante se destruye
  (Actor|DestroyActor))

(event EventBeginPlay
  ;[1 1 1] Pasado cierto tiempo, la bomba gigante se destruye
  (Utilities|Time|SetTimerbyEvent (delegate Custom|morir) (Variables|Default|GettiempoDeExistencia)))

(event EventTick
  (params (DeltaSeconds :type Float%20%28single-precision%29))
  ;[1 1 1] Actualizamos la bomba gigante (su transform)
  (CallFunction|FuncActualizar DeltaSeconds))

(fn ConstructionScript)

(fn FuncActualizar
  (params (delta :type Float%20%28single-precision%29))
  (bind _malla_bomba (Variables|Default|Getmalla_bomba))
  (bind _returnvalue (Transformation|GetWorldLocation _malla_bomba))
  ;[1 1 1] Se aumenta el tamaño de la bomba gigante
  (CallFunction|FuncAumentarTamaño delta)
  ;[1 1 1] Se calcula una nueva posición para que la bomba gigante se desplace hacia el fondo del túnel
  (bind _asbp_nave (Utilities|Casting|CastToBP_nave (Game|Player|GetPlayerPawn 0)))
  (bind (_nuevax _nuevaz) (CallFunction|FuncLlevarACentro (.x _returnvalue) (.z _returnvalue) delta))
  (Transformation|SetWorldLocation _malla_bomba (Math|Vector|MakeVector _nuevax (+ (.y _returnvalue) (* delta (Variables|/Game/BluePrints/BP_nave.BP_nave_C|GetmaxVelocidadY _asbp_nave)) (Variables|Default|Getvelocidad)) _nuevaz) false false)
  ;[1 1 1] Se rota la bomba gigante respecto a su eje Z (eje Y del mundo)
  (Transformation|AddLocalRotation (Variables|Default|Getmalla_bomba) (Math|Rotator|MakeRotator 0.0 0.0 (* (Variables|Default|GetvelocidadRotacion) delta)) false false))

(fn FuncLlevarACentro
  (params (X :type Float%20%28single-precision%29) (Z :type Float%20%28single-precision%29) (delta :type Float%20%28single-precision%29))
  (bind _returnvalue (Math|Vector2D|MakeVector2D X Z))
  (bind _velocidadacentro (Variables|Default|GetvelocidadACentro))
  (bind _returnvalue_2 (* _returnvalue _velocidadacentro))
  (bind _returnvalue_3 (* _returnvalue_2 delta))
  (bind _returnvalue_4 (- _returnvalue _returnvalue_3))
  ;[1 1 1] Se lleva la bomba gigante hacia el centro del túnel poco a poco
  (return (.x _returnvalue_4) (.y _returnvalue_4)))

(fn FuncAumentarTamaño
  (params (delta :type Float%20%28single-precision%29))
  (bind _tamañomaximo (Variables|Default|GettamañoMaximo))
  (bind _velocidadescalado (Variables|Default|GetvelocidadEscalado))
  (bind _malla_bomba (Variables|Default|Getmalla_bomba))
  (bind _returnvalue (Transformation|GetWorldScale _malla_bomba))
  (bind _returnvalue_2 (* _velocidadescalado delta))
  (bind _returnvalue_3 (+ _returnvalue _returnvalue_2))
  (bind _returnvalue_4 (Math|Float|Clamp(Float) (.x _returnvalue_3) 0.0 _tamañomaximo))
  ;[1 1 1] Se aumenta el tamaño de la bomba gigante para que ocupe todo el ancho del túnel hasta un máximo establecido
  (Transformation|SetWorldScale3D _malla_bomba (Math|Vector|MakeVector _returnvalue_4 _returnvalue_4 _returnvalue_4)))