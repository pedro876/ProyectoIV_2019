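; Enemy turret that tracks and shoots the player ship (BP_nave), with a function to randomly hide it.
; Tick drives a rest/turn/attack/death state machine, engaging by Y distance and resting once passed.
; Turning pitches the body by signed plane-projected angle, clamped if grounded, while the gun aims directly.
; Attack spawns BP_bala on a looping timer, returning to turning when the ship leaves the firing arc, unless Bloqueado (grounded, ship not above).
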(event Custom|evento_empezarAtaque
  ;[1 1 1] Eventos del estado de ataque
  (bind _returnvalue (Utilities|Time|SetTimerbyEvent (delegate Custom|evento_disparar) 1.0 true)))

(event Custom|evento_disparar
  ;[1 1 1] Eventos del estado de ataque
  (bind _empezargiro (CallFunction|FuncDisparar))
  (if _empezargiro
    (Utilities|Time|ClearandInvalidateTimerbyHandle (stale Custom|evento_empezarAtaque _returnvalue))
    (CallFunction|FuncCambiarEstado "NewEnumerator1")))

(event EventTick
  (params (DeltaSeconds :type Float%20%28single-precision%29))
  (CallFunction|FuncActualizarEstado DeltaSeconds)
  (CallFunction|FuncComprobarDistanciaAtaque))

(fn ConstructionScript)

(fn FuncAleatorizar
  (params (enElSuelo :type Boolean))
  (Variables|Default|SetenElSuelo enElSuelo)
  (if (< (Math|Random|RandomFloat) (Variables|Default|Getprobabilidad_destruir))
    (Rendering|SetActorHiddenInGame true)
    (Collision|SetActorEnableCollision false)
    (else
      (Rendering|SetActorHiddenInGame false)
      (Collision|SetActorEnableCollision true)))
  (CallFunction|FuncCambiarEstado "NewEnumerator2"))

(fn FuncActualizarEstado
  (params (delta :type Float%20%28single-precision%29))
  (if (not (or (Variables|Rendering|GetbHidden) (Variables|/Script/Engine.Actor|GetbHidden (Actor|GetParentActor))))
    (switch Utilities|FlowControl|Switch|SwitchonestadosEnemigo (Variables|Default|GetestadoActual)
      (:NewEnumerator0
        _)
      (:NewEnumerator1
        (CallFunction|FuncEstadoGirar delta)))
    (CallFunction|FuncApuntarPistola)))

(fn FuncCambiarEstado
  (params (estadoNuevo :type estadosEnemigo%20Enum :default "NewEnumerator2"))
  (switch Utilities|FlowControl|Switch|SwitchonestadosEnemigo estadoNuevo
    (:NewEnumerator0
      (if (or (Utilities|Enum|Equal(Enum) (Variables|Default|GetestadoActual) "NewEnumerator2") (Utilities|Enum|Equal(Enum) (Variables|Default|GetestadoActual) "NewEnumerator1"))
        (Variables|Default|SetestadoActual estadoNuevo)
        (CallFunction|EventoEmpezarAtaque)))
    (:NewEnumerator1
      (if (or (Utilities|Enum|Equal(Enum) (Variables|Default|GetestadoActual) "NewEnumerator2") (Utilities|Enum|Equal(Enum) (Variables|Default|GetestadoActual) "NewEnumerator0"))
        (Variables|Default|SetestadoActual estadoNuevo)))
    (:NewEnumerator2
      (Variables|Default|SetestadoActual estadoNuevo))
    (:NewEnumerator3
      (Variables|Default|SetestadoActual estadoNuevo))))

(fn FuncEstadoGirar
  (params (delta :type Float%20%28single-precision%29))
  (bind _bloqueado (Variables|Default|Getbloqueado))
  ;[1 1 1] Actualizar rotación
  (bind _angulo (CallFunction|FuncAnguloANave))
  (Transformation|AddWorldRotation (Variables|Default|Getmalla_enemigo) (Math|Rotator|MakeRotator 0.0 (* _angulo (* delta (Variables|Default|GetvelocidadGiro))) 0.0) false false)
  (CallFunction|FuncLimitarRotacion)
  (bind _fueraderango (CallFunction|FuncFueraDeRango _angulo))
  (Development|PrintString (Utilities|String|ToString(Boolean) _bloqueado))
  (if (not (and _fueraderango (not _bloqueado)))
    (CallFunction|FuncCambiarEstado "NewEnumerator0")))

(fn FuncAnguloANave
  (bind _malla_enemigo (Variables|Default|Getmalla_enemigo))
  (bind _returnvalue (Math|Vector|GetUpVector _malla_enemigo))
  (bind _direccion (CallFunction|FuncDireccionANave (Variables|Default|Getmalla_enemigo)))
  (return (* (Class|KismetMathLibrary|DegAcos (Math|Vector|DotProduct (Math|Vector|Normalize (Math|Vector|ProjectVectorontoPlane _direccion "0,-1.000000,0.000000")) _returnvalue)) (Math|Float|Sign(Float) (.y (Math|Vector|CrossProduct (Math|Vector|Normalize (Math|Vector|ProjectVectorontoPlane _direccion "0,-1.000000,0.000000")) _returnvalue))))))

(fn FuncDisparar
  (Game|SpawnActorfromClass "/Game/BluePrints/BP_bala.BP_bala_C" (Transformation|GetWorldTransform (Variables|Default|GetorigenBala)) "Undefined" 0 0)
  ;[1 1 1] Comprobar si está fuera del rango
  (bind _angulo (CallFunction|FuncAnguloANave))
  (bind _fueraderango (CallFunction|FuncFueraDeRango _angulo))
  (bind _asbp_nave (Utilities|Casting|CastToBP_nave (Game|Player|GetPlayerPawn 0)))
  ;[1 1 1] Si la nave está por encima del enemigo lo desbloqueo
  (bind _output_get (Variables|Default|Setbloqueado (and (Variables|Default|GetenElSuelo) (<= (.z (Transformation|GetWorldLocation (Variables|/Game/BluePrints/BP_nave.BP_nave_C|GetcolisionNave _asbp_nave))) (.z (Transformation|GetWorldLocation (Variables|Default|Getmalla_enemigo)))))))
  (return (and (not _output_get) _fueraderango)))

(fn FuncFueraDeRango
  (params (angulo :type Float%20%28single-precision%29))
  (return (not (< (Math|Float|Absolute(Float) angulo) (/ (Variables|Default|GetrangoParaDisparar) 2.0)))))

(fn FuncDireccionANave
  (params (origen :type Static%20Mesh%20Component%20Object%20Reference))
  (bind _asbp_nave (Utilities|Casting|CastToBP_nave (Game|Player|GetPlayerPawn 0)))
  (return (- (Transformation|GetWorldLocation (Variables|/Game/BluePrints/BP_nave.BP_nave_C|GetcolisionNave _asbp_nave)) (Transformation|GetWorldLocation origen))))

(fn FuncLimitarRotacion
  (bind _malla_enemigo (Variables|Default|Getmalla_enemigo))
  (if (Variables|Default|GetenElSuelo)
    (Transformation|SetWorldRotation _malla_enemigo (Math|Rotator|MakeRotator 0.0 (Math|Float|ClampAngle (.pitch (Transformation|GetWorldRotation _malla_enemigo)) -69.0 69.0) 1.8e+02) false false)))

(fn FuncComprobarDistanciaAtaque
  (bind _malla_enemigo (Variables|Default|Getmalla_enemigo))
  (bind _returnvalue (Transformation|GetWorldLocation _malla_enemigo))
  (bind _asbp_nave (Utilities|Casting|CastToBP_nave (Game|Player|GetPlayerPawn 0)))
  ;[1 1 1] Si la nave ha dejado atrás al enemigo
  (if (< (.y (Transformation|GetWorldLocation (Variables|/Game/BluePrints/BP_nave.BP_nave_C|GetcolisionNave _asbp_nave))) (.y _returnvalue))
    (CallFunction|FuncCambiarEstado "NewEnumerator2")
    (Variables|Default|SetnaveEnRango false)
    (elif (and (<= (Math|Float|Absolute(Float) (- (.y (Transformation|GetWorldLocation (Variables|/Game/BluePrints/BP_nave.BP_nave_C|GetcolisionNave _asbp_nave))) (.y _returnvalue))) (Variables|Default|GetdistanciaDeAtaque)) (not (Variables|Default|GetnaveEnRango)))
      (CallFunction|FuncCambiarEstado "NewEnumerator1")
      (Variables|Default|SetnaveEnRango true))))

(fn FuncApuntarPistola
  (bind _asbp_nave (Utilities|Casting|CastToBP_nave (Game|Player|GetPlayerPawn 0)))
  (Transformation|SetWorldRotation (Variables|Default|Getmalla_pistola) (Math|Rotator|FindLookatRotation (Transformation|GetWorldLocation (Variables|Default|Getmalla_pistola)) (Transformation|GetWorldLocation (Variables|/Game/BluePrints/BP_nave.BP_nave_C|GetcolisionNave _asbp_nave))) false false))